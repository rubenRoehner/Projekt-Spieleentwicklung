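; End-wall door for the Level 1 subway train that slides open and then switches the player's view.
; OpenDoor plays a timeline that moves the door mesh along X and flags it open, then after a short delay blends the view target to another camera.
; A box trigger shows an interaction prompt widget and a hint actor to Louri while the door is closed, removing both on exit.
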(event OnComponentEndOverlap(Box)
  (params (OverlappedComponent :type Primitive%20Component%20Object%20Reference) (OtherActor :type Actor%20Object%20Reference) (OtherComp :type Primitive%20Component%20Object%20Reference) (OtherBodyIndex :type Integer))
  ;[1 1 1] Box Collision
  (Utilities|Casting|CastToLouri OtherActor)
  ;[1 1 1] Add and remove interaction prompt
  (Widget|RemovefromParent (stale OnComponentBeginOverlap(Box) _returnvalue))
  (Rendering|SetActorHiddenInGame (Variables|Default|GetHint) true))

(event OnComponentBeginOverlap(Box)
  (params (OverlappedComponent :type Primitive%20Component%20Object%20Reference) (OtherActor :type Actor%20Object%20Reference) (OtherComp :type Primitive%20Component%20Object%20Reference) (OtherBodyIndex :type Integer) (bFromSweep :type Boolean) (SweepResult :type Hit%20Result%20Structure%20%28by%20ref%29))
  ;[1 1 1] Box Collision
  (Utilities|Casting|CastToLouri OtherActor)
  (if (not (Variables|Default|GetIsDoorOpen))
    ;[1 1 1] Add and remove interaction prompt
    (bind _returnvalue (UserInterface|CreateWidget "/Game/Level/Level_1/InteractPrompDoor.InteractPrompDoor_C"))
    (UserInterface|Viewport|AddtoViewport _returnvalue 0)
    (Rendering|SetActorHiddenInGame (Variables|Default|GetHint) false)))

(event Custom|Open%20Door
  (bind _open_track (Timeline|Timeline_0 Play)
    (:Update
      (Transformation|SetRelativeLocation (Variables|Default|Getendwall_door_01) (Math|Vector|Lerp(Vector) "5.000000,0.000000, 0" "75.000000,0.000000, 0" _open_track) false false)
      (Variables|Default|SetIsDoorOpen true))
    (:Finished
      (Utilities|FlowControl|Delay 1.0)
      (Game|Player|SetViewTargetwithBlend (Game|GetPlayerController 0) (Variables|Default|GetCameraToFInd) 0.0 "VTBlend_Linear" 0.0 false))))

(fn ConstructionScript)
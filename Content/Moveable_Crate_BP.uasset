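; Pushable crate that enables physics on its mesh and sets Louri's IsPushing while Louri overlaps either axis trigger.
; Construction script adds an arrow for each PushTransforms entry.
; An interaction path looks up the character's PushComponent and nearest push transform within PushRange, but OnInteracted passes no character and the search receives the forward vector as location.
; The clearance, floor and wall checks, teleport and BeginPush are disconnected, so never run.
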(event OnComponentBeginOverlap(Y-AxisCollision)
  (params (OverlappedComponent :type Primitive%20Component%20Object%20Reference) (OtherActor :type Actor%20Object%20Reference) (OtherComp :type Primitive%20Component%20Object%20Reference) (OtherBodyIndex :type Integer) (bFromSweep :type Boolean) (SweepResult :type Hit%20Result%20Structure%20%28by%20ref%29))
  ;[1 1 1] Y-Axis Collision
  (bind _aslouri (Utilities|Casting|CastToLouri OtherActor))
  (Variables|/Game/Character/Louri/Louri.Louri_C|SetIsPushing _aslouri true)
  (Physics|SetSimulatePhysics (Variables|Default|GetCrate) true))

(event OnComponentBeginOverlap(X-AxisCollision)
  (params (OverlappedComponent :type Primitive%20Component%20Object%20Reference) (OtherActor :type Actor%20Object%20Reference) (OtherComp :type Primitive%20Component%20Object%20Reference) (OtherBodyIndex :type Integer) (bFromSweep :type Boolean) (SweepResult :type Hit%20Result%20Structure%20%28by%20ref%29))
  ;[1 1 1] X-Axis Collision
  (bind _aslouri (Utilities|Casting|CastToLouri OtherActor))
  (Variables|/Game/Character/Louri/Louri.Louri_C|SetIsPushing _aslouri true)
  (Physics|SetSimulatePhysics (Variables|Default|GetCrate) true))

(event OnComponentEndOverlap(Y-AxisCollision)
  (params (OverlappedComponent :type Primitive%20Component%20Object%20Reference) (OtherActor :type Actor%20Object%20Reference) (OtherComp :type Primitive%20Component%20Object%20Reference) (OtherBodyIndex :type Integer))
  ;[1 1 1] Y-Axis Collision
  (bind _aslouri (Utilities|Casting|CastToLouri OtherActor))
  (Variables|/Game/Character/Louri/Louri.Louri_C|SetIsPushing _aslouri false)
  (Physics|SetSimulatePhysics (Variables|Default|GetCrate) false))

(event OnComponentEndOverlap(X-AxisCollision)
  (params (OverlappedComponent :type Primitive%20Component%20Object%20Reference) (OtherActor :type Actor%20Object%20Reference) (OtherComp :type Primitive%20Component%20Object%20Reference) (OtherBodyIndex :type Integer))
  ;[1 1 1] X-Axis Collision
  (bind _aslouri (Utilities|Casting|CastToLouri OtherActor))
  (Variables|/Game/Character/Louri/Louri.Louri_C|SetIsPushing _aslouri false)
  (Physics|SetSimulatePhysics (Variables|Default|GetCrate) false))

(event EventOnInteracted
  (params (Player :type Louri%20Object%20Reference))
  (CallFunction|HandleInteraction))

(fn ConstructionScript
  (for _array_element (Variables|Default|GetPushTransforms)
    (AddComponent|AddArrowComponent false _array_element)))

(fn HandleInteraction
  (params (Character :type Character%20Object%20Reference))
  (Utilities|IsValid Character
    (:Is%20Valid
      (bind _output_get (LocalVariables|SetPushComponent (Actor|GetComponentbyClass Character "/Game/PushComponent.PushComponent_C")))
      (Utilities|IsValid _output_get
        (:Is%20Valid
          (bind _bestindex (CallFunction|FindClosestPushTransformIndex (Math|Conversions|ToVector2D(Vector) (Transformation|GetActorForwardVector Character)) (Variables|Default|GetPushRange))))
        (:Is%20Not%20Valid
          (Utilities|PushFailedInfo "Character does not have push component"))))
    (:Is%20Not%20Valid
      (Utilities|PushFailedInfo "Character is invalid"))))

(fn FindClosestPushTransformIndex
  (params (CharacterLocation :type Vector%202D%20Structure) (PushRange :type Float%20%28double-precision%29))
  (for (_array_element _array_index) (Variables|Default|GetPushTransforms)
    (LocalVariables|SetCurrentTransformIndex _array_index)
    (bind _output_get (LocalVariables|SetCurrentDistanceSq (Class|KismetMathLibrary|DistanceSquared2D (Math|Conversions|ToVector2D(Vector) (Math|Transform|TransformLocation (Transformation|GetActorTransform) (.location _array_element))) CharacterLocation)))
    (if (< _output_get (Math|Float|Square PushRange))
      (if (or (< (LocalVariables|GetCurrentDistanceSq) (LocalVariables|GetClosestDistanceSq)) (< (LocalVariables|GetClosestTransformIndex) 0))
        (LocalVariables|SetClosestTransformIndex (LocalVariables|GetCurrentTransformIndex))
        (LocalVariables|SetClosestDistanceSq (LocalVariables|GetCurrentDistanceSq)))))
  (return (LocalVariables|GetClosestTransformIndex)))
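; BP_Door_double_01 is a sliding double door in the subway train level that opens when its OpenDoor event is called.
; Two timelines started from a Sequence lerp the relative locations of the left and right door meshes, sliding them apart along X.
; One second after the left door finishes, the first player controller's view target is set to CameraToFInd.
; The blueprint has no closing logic.
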(event Custom|Open%20Door
  (Utilities|FlowControl|Sequence
    (:then_0
      (bind _open_track (Timeline|OpenDoor%20TImeLine Play)
        (:Update
          ;[1 1 1] Open Left Door
          (Transformation|SetRelativeLocation (Variables|Default|Getwall_doorway_door_02) (Math|Vector|Lerp(Vector) "-150.000000,1.000000, 0" "-210.000000,1.000000, 0" _open_track) false false))
        (:Finished
          (Utilities|FlowControl|Delay 1.0)
          (Game|Player|SetViewTargetwithBlend (Game|GetPlayerController 0) (Variables|Default|GetCameraToFInd) 0.0 "VTBlend_Linear" 0.0 false))))
    (:then_1
      (bind _open_track_2 (Timeline|Timeline_0 Play)
        (:Update
          ;[1 1 1] Open Right Door
          (Transformation|SetRelativeLocation (Variables|Default|Getwall_doorway_door_01) (Math|Vector|Lerp(Vector) "0,1.000000, 0" "60.000000,1.000000, 0" _open_track_2) false false))))))

(fn ConstructionScript)